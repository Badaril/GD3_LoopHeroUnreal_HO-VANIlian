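; BP_MazeCell runs a maze quest segment that hands control to a separate character and camera, then returns it to the player's original pawn.
; Activate, blocked once the quest is finished, switches possession, view target and adds the maze input mapping.
; QuitMaze restores pawn and camera, adds the pawn's mapping and teleports the maze character to its saved start.
; It then marks the quest finished if the game instance has the ring, otherwise reactivates the ring.
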(event EventBeginPlay
  (|CallParentFunction)
  (bind _asbp_loop_game_instance (Utilities|Casting|CastToBP_LoopGameInstance (Game|GetGameInstance)))
  (Variables|Default|SetAs%20BP%20Loop%20Game%20Instance _asbp_loop_game_instance)
  (Variables|Default|SetStartingPoint (Transformation|GetActorTransform (Variables|Default|GetNewPlayerCharacter))))

(event Collision|EventActorBeginOverlap
  (params (OtherActor :type Actor%20Object%20Reference))
  (|CallParentFunction OtherActor) ; This node is disabled and will not be called.\nDrag off pins to build functionality.
)

(event EventTick
  (params (DeltaSeconds :type Float%20%28single-precision%29))
  (|CallParentFunction DeltaSeconds) ; This node is disabled and will not be called.\nDrag off pins to build functionality.
)

(event EventActivate
  (params (Pawn :type BP%20Player%20Pawn%20Object%20Reference))
  (if (not (Variables|/Game/Blueprints/Global/BP_LoopGameInstance.BP_LoopGameInstance_C|GetIsQuestFinished (Variables|Default|GetAs%20BP%20Loop%20Game%20Instance)))
    (Pawn|Possess (Game|GetPlayerController 0) (Variables|Default|GetNewPlayerCharacter))
    (Game|Player|SetViewTargetwithBlend (Game|GetPlayerController 0) (Variables|Default|GetMazeCam) 0.0 "VTBlend_Linear" 0.0 false)
    (Input|AddMappingContext (PlayerController|LocalPlayerSubsystems|GetEnhancedInputLocalPlayerSubsystem (Game|GetPlayerController 0)) "/Game/ThirdPerson/Input/IMC_Default.IMC_Default" 0 "(bIgnoreAllPressedKeysUntilRelease=True,bForceImmediately=False,bNotifyUserSettings=False)")))

(fn ConstructionScript
  (|CallParentFunction))

(fn QuitMaze
  (Pawn|Possess (Game|GetPlayerController 0) (Variables|Default|GetOldCharacterPawn))
  (Game|Player|SetViewTargetwithBlend (Game|GetPlayerController 0) (Variables|Default|GetPlayerCam) 0.0 "VTBlend_Linear" 0.0 false)
  (Input|AddMappingContext (PlayerController|LocalPlayerSubsystems|GetEnhancedInputLocalPlayerSubsystem (Game|GetPlayerController 0)) "/Game/Blueprints/Global/IMC_PlayerPawn.IMC_PlayerPawn" 0 "(bIgnoreAllPressedKeysUntilRelease=True,bForceImmediately=False,bNotifyUserSettings=False)")
  (Transformation|SetActorTransform (Variables|Default|GetNewPlayerCharacter) (Variables|Default|GetStartingPoint) false true)
  (if (Variables|/Game/Blueprints/Global/BP_LoopGameInstance.BP_LoopGameInstance_C|GetHasRing (Variables|Default|GetAs%20BP%20Loop%20Game%20Instance))
    (Variables|/Game/Blueprints/Global/BP_LoopGameInstance.BP_LoopGameInstance_C|SetIsQuestFinished (Variables|Default|GetAs%20BP%20Loop%20Game%20Instance) true)
    (else
      (Default|SetActive (Variables|Default|GetRingRef) true))))