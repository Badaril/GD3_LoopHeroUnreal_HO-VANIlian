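; Fighting cell that stages an automatic fight between the player and its monster, switching to a combat camera and HUD on activation.
; Each Tick, the player attacks when stamina reaches a threshold and the monster retaliates, both through damage components gated by attack cooldowns, updating health displays.
; Activation resets stamina and registers the cell with both damage components; FightOver restores the player camera and HUD.
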(event EventTick
  (params (DeltaSeconds :type Float%20%28single-precision%29))
  (|CallParentFunction DeltaSeconds)
  (if (Variables|Default|GetFight)
    (Default|UpdateStamina (Variables|/Game/Blueprints/Gameplay/BP_PlayerPawn.BP_PlayerPawn_C|GetPlayerHUD (Variables|Default|GetPlayerRef)) (Variables|/Game/Blueprints/Global/BP_LoopGameInstance.BP_LoopGameInstance_C|GetPlayerStamina (Variables|/Game/Blueprints/Gameplay/BP_PlayerPawn.BP_PlayerPawn_C|GetAs%20BP%20Loop%20Game%20Instance (Variables|Default|GetPlayerRef))))
    (if (and (>= (Variables|/Game/Blueprints/Global/BP_LoopGameInstance.BP_LoopGameInstance_C|GetPlayerStamina (Variables|/Game/Blueprints/Gameplay/BP_PlayerPawn.BP_PlayerPawn_C|GetAs%20BP%20Loop%20Game%20Instance (Variables|Default|GetPlayerRef))) 6e+01) (not (Variables|/Game/Blueprints/Global/Components/BPC_Damage.BPC_Damage_C|GetAttackCooldown (Variables|/Game/Blueprints/Gameplay/BP_PlayerPawn.BP_PlayerPawn_C|GetBPC_Damage (Variables|Default|GetPlayerRef)))))
      (Default|DealDamage (Variables|/Game/Blueprints/Gameplay/BP_PlayerPawn.BP_PlayerPawn_C|GetBPC_Damage (Variables|Default|GetPlayerRef)) (Variables|/Game/Blueprints/Gameplay/BP_Monster.BP_Monster_C|GetBPC_Damage (Variables|Default|GetMonsterRef)))
      (Utilities|IsValid (Variables|Default|GetMonsterRef)
        (:Is%20Valid
          (Default|UpdateHealth (Variables|Default|GetAs%20WBP%20Health%20Bar) (Variables|/Game/Blueprints/Global/Components/BPC_Damage.BPC_Damage_C|GetHealth (Variables|/Game/Blueprints/Gameplay/BP_Monster.BP_Monster_C|GetBPC_Damage (Variables|Default|GetMonsterRef)))))))
    (if (not (Variables|/Game/Blueprints/Global/Components/BPC_Damage.BPC_Damage_C|GetAttackCooldown (Variables|/Game/Blueprints/Gameplay/BP_Monster.BP_Monster_C|GetBPC_Damage (Variables|Default|GetMonsterRef))))
      (Default|DealDamage (Variables|/Game/Blueprints/Gameplay/BP_Monster.BP_Monster_C|GetBPC_Damage (Variables|Default|GetMonsterRef)) (Variables|/Game/Blueprints/Gameplay/BP_PlayerPawn.BP_PlayerPawn_C|GetBPC_Damage (Variables|Default|GetPlayerRef)))
      (Default|UpdateHealth (Variables|/Game/Blueprints/Gameplay/BP_PlayerPawn.BP_PlayerPawn_C|GetPlayerHUD (Variables|Default|GetPlayerRef)) (Variables|/Game/Blueprints/Global/Components/BPC_Damage.BPC_Damage_C|GetHealth (Variables|/Game/Blueprints/Gameplay/BP_PlayerPawn.BP_PlayerPawn_C|GetBPC_Damage (Variables|Default|GetPlayerRef)))))))

(event EventActivate
  (params (Pawn :type BP%20Player%20Pawn%20Object%20Reference))
  (Utilities|IsValid (Variables|Default|GetMonsterRef)
    (:Is%20Valid
      (Default|UpdateHealth (Variables|Default|GetAs%20WBP%20Health%20Bar) 1e+01)
      (Variables|Default|SetPlayerRef Pawn)
      (Variables|/Game/Blueprints/Global/Components/BPC_Damage.BPC_Damage_C|SetFightingCell (Variables|/Game/Blueprints/Gameplay/BP_PlayerPawn.BP_PlayerPawn_C|GetBPC_Damage (Variables|Default|GetPlayerRef)) self)
      (Variables|/Game/Blueprints/Global/Components/BPC_Damage.BPC_Damage_C|SetFightingCell (Variables|/Game/Blueprints/Gameplay/BP_Monster.BP_Monster_C|GetBPC_Damage (Variables|Default|GetMonsterRef)) self)
      (Game|Player|SetViewTargetwithBlend (Game|GetPlayerController 0) (Variables|Default|GetFightingCam) 0.0 "VTBlend_Linear" 0.0 false)
      (Variables|Default|SetFight true)
      (Variables|/Game/Blueprints/Global/BP_LoopGameInstance.BP_LoopGameInstance_C|SetPlayerStamina (Variables|/Game/Blueprints/Gameplay/BP_PlayerPawn.BP_PlayerPawn_C|GetAs%20BP%20Loop%20Game%20Instance (Variables|Default|GetPlayerRef)) 0.0)
      (Default|SetFightingHUD (Variables|/Game/Blueprints/Gameplay/BP_PlayerPawn.BP_PlayerPawn_C|GetPlayerHUD (Variables|Default|GetPlayerRef)) true)
      (Variables|/Game/Blueprints/Gameplay/BP_Monster.BP_Monster_C|SetIsAttacking (Variables|Default|GetMonsterRef) true))))

(event EventBeginPlay
  (bind _aswbp_health_bar (Utilities|Casting|CastToWBP_HealthBar (UserInterface|GetWidget (Variables|/Game/Blueprints/Gameplay/BP_HealthBarInWorld.BP_HealthBarInWorld_C|GetWidget (Variables|Default|GetMonsterHealthDisplay)))))
  (Variables|Default|SetAs%20WBP%20Health%20Bar _aswbp_health_bar))

(fn ConstructionScript
  (|CallParentFunction))

(fn FightOver
  (Variables|Default|SetFight false)
  (Game|Player|SetViewTargetwithBlend (Game|GetPlayerController 0) (Variables|Default|GetPlayerCam) 0.0 "VTBlend_Linear" 0.0 false)
  (Default|SetFightingHUD (Variables|/Game/Blueprints/Gameplay/BP_PlayerPawn.BP_PlayerPawn_C|GetPlayerHUD (Variables|Default|GetPlayerRef)) false))