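; BP_TrapCell is a trap cell that changes the player's health when activated with a pawn.
; Activate adds its Value to PlayerHealth on the pawn's BPLoopGameInstance reference and clamps the result to a fixed range.
; It then pushes the new health to the pawn's PlayerHUD.
; Begin play, overlap and tick are disabled stubs, so all behavior runs through Activate.
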(event EventBeginPlay
  (|CallParentFunction) ; This node is disabled and will not be called.\nDrag off pins to build functionality.
)

(event Collision|EventActorBeginOverlap
  (params (OtherActor :type Actor%20Object%20Reference))
  (|CallParentFunction OtherActor) ; This node is disabled and will not be called.\nDrag off pins to build functionality.
)

(event EventTick
  (params (DeltaSeconds :type Float%20%28single-precision%29))
  (|CallParentFunction DeltaSeconds) ; This node is disabled and will not be called.\nDrag off pins to build functionality.
)

(event EventActivate
  (params (Pawn :type BP%20Player%20Pawn%20Object%20Reference))
  (bind _as_bp_loop_game_instance (Variables|/Game/Blueprints/Gameplay/BP_PlayerPawn.BP_PlayerPawn_C|GetAs%20BP%20Loop%20Game%20Instance Pawn))
  (bind _output_get (Variables|/Game/Blueprints/Global/BP_LoopGameInstance.BP_LoopGameInstance_C|SetPlayerHealth _as_bp_loop_game_instance (Math|Float|Clamp(Float) (+ (Variables|/Game/Blueprints/Global/BP_LoopGameInstance.BP_LoopGameInstance_C|GetPlayerHealth _as_bp_loop_game_instance) (Variables|Default|GetValue)) 0.0 2e+01)))
  (Default|UpdateHeath (Variables|/Game/Blueprints/Gameplay/BP_PlayerPawn.BP_PlayerPawn_C|GetPlayerHUD Pawn) _output_get))

(fn ConstructionScript
  (|CallParentFunction))