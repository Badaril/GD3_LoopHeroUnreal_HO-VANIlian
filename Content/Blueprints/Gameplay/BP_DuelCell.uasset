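; BP_DuelCell is a cell that starts a duel when activated, apparently as part of a board.
; Activate creates the WBP_DuelBackground widget, adds it to the player's screen and focuses it in Game and UI input mode.
; DuelOver calls UpdateParkour on the board if the player has won, then removes the widget in either case.
; BeginPlay caches the BP_LoopGameInstance reference.
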(event EventBeginPlay
  (|CallParentFunction)
  (bind _asbp_loop_game_instance (Utilities|Casting|CastToBP_LoopGameInstance (Game|GetGameInstance)))
  (Variables|Default|SetAs%20BP%20Loop%20Game%20Instance _asbp_loop_game_instance))

(event Collision|EventActorBeginOverlap
  (params (OtherActor :type Actor%20Object%20Reference))
  (|CallParentFunction OtherActor) ; This node is disabled and will not be called.\nDrag off pins to build functionality.
)

(event EventTick
  (params (DeltaSeconds :type Float%20%28single-precision%29))
  (|CallParentFunction DeltaSeconds))

(event EventActivate
  (params (Pawn :type BP%20Player%20Pawn%20Object%20Reference))
  (bind _returnvalue (UserInterface|CreateWidget "/Game/Blueprints/UI/WBP_DuelBackground.WBP_DuelBackground_C"))
  (bind _output_get (Variables|Default|SetDuelHUDRef _returnvalue))
  (UserInterface|Viewport|AddtoPlayerScreen _output_get)
  (Input|SetInputModeGameandUI (Game|GetPlayerController 0) (Variables|Default|GetDuelHUDRef) "DoNotLock" true false))

(fn ConstructionScript
  (|CallParentFunction))

(fn DuelOver
  (if (Variables|Default|GetPlayerHasWin)
    (Default|UpdateParkour (Variables|Default|GetBoardRef)))
  (Widget|RemovefromParent (Variables|Default|GetDuelHUDRef)))