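; Player pawn for a cell-based board, with its current cell number stored in BP_LoopGameInstance.
; TryMoving adds a value to that number, resolves the next cell through the Board, saves it and calls MoveToCell.
; MoveToCell teleports straight to the saved cell's transform and advances PawnPosition by one, wrapping at the cell count.
; Tick repeats MoveToCell until PawnPosition matches the saved number.
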(event EventBeginPlay
  (bind _asbp_loop_game_instance (Utilities|Casting|CastToBP_LoopGameInstance (Game|GetGameInstance)))
  (Variables|Default|SetAs%20BP%20Loop%20Game%20Instance _asbp_loop_game_instance))

(event Collision|EventActorBeginOverlap
  (params (OtherActor :type Actor%20Object%20Reference)))

(event EventTick
  (params (DeltaSeconds :type Float%20%28single-precision%29))
  (if (!= (Variables|Default|GetPawnPosition) (Variables|/Game/Blueprints/Global/BP_LoopGameInstance.BP_LoopGameInstance_C|GetCellNumber (Variables|Default|GetAs%20BP%20Loop%20Game%20Instance)))
    (CallFunction|MovetoCell)))

(fn ConstructionScript)

(fn MovetoCell
  (bind _cell (Default|GetCellbyNumber (Variables|Default|GetBoard) (Variables|/Game/Blueprints/Global/BP_LoopGameInstance.BP_LoopGameInstance_C|GetCellNumber (Variables|Default|GetAs%20BP%20Loop%20Game%20Instance))))
  (Transformation|SetActorTransform (Transformation|GetActorTransform _cell) false true)
  (bind _result (Math|Integer|IncrementInt (Variables|Default|GetPawnPosition))
    (:%20%20
      (Variables|Default|SetPawnPosition (Math|Integer|%(Integer) _result (Utilities|Array|Length (Variables|/Game/Blueprints/Gameplay/BP_Board.BP_Board_C|GetCells (Variables|Default|GetBoard))))))))

(fn TryMoving
  (params (Value :type Integer))
  (bind _newcellnumber (Default|GetNextCelltoMove (Variables|Default|GetBoard) (+ (Variables|/Game/Blueprints/Global/BP_LoopGameInstance.BP_LoopGameInstance_C|GetCellNumber (Variables|Default|GetAs%20BP%20Loop%20Game%20Instance)) Value)))
  (Variables|/Game/Blueprints/Global/BP_LoopGameInstance.BP_LoopGameInstance_C|SetCellNumber (Variables|Default|GetAs%20BP%20Loop%20Game%20Instance) _newcellnumber)
  (CallFunction|MovetoCell))