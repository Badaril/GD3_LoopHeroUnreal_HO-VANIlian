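; Dice actor that produces a random value and passes it to the player pawn to attempt a move.
; On BeginPlay, after a short delay, it registers itself in the player HUD as the D6 or D3 die, depending on MaxValue.
; IsRolling randomizes Value between one and MaxValue, while RollDice only sends the current Value to the pawn's TryMoving.
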(event EventBeginPlay
  (bind _playerpawn (Variables|Default|GetPlayerPawn))
  (bind _playerhud (Variables|/Game/Blueprints/Gameplay/BP_PlayerPawn.BP_PlayerPawn_C|GetPlayerHUD _playerpawn))
  (Utilities|FlowControl|Delay 0.2)
  (if (>= (Variables|Default|GetMaxValue) 4)
    (Variables|/Game/Blueprints/UI/WBP_PlayerHUD.WBP_PlayerHUD_C|SetDice_D6 _playerhud self)
    (else
      (Variables|/Game/Blueprints/UI/WBP_PlayerHUD.WBP_PlayerHUD_C|SetDice_D3 _playerhud self))))

(event Collision|EventActorBeginOverlap
  (params (OtherActor :type Actor%20Object%20Reference)))

(event EventTick
  (params (DeltaSeconds :type Float%20%28single-precision%29)))

(fn ConstructionScript)

(fn RollDice
  (Default|TryMoving (Variables|Default|GetPlayerPawn) (Variables|Default|GetValue)))

(fn IsRolling
  (Variables|Default|SetValue (Math|Random|RandomIntegerinRange 1 (Variables|Default|GetMaxValue))))