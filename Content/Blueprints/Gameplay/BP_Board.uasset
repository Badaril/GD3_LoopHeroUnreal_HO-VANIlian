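; BP_Board holds the ordered list of cells that forms a board route, with lookup by number.
; GetNextCellToMove wraps a cell number around the array length, so the route loops.
; UpdateParkour displays the MazePath, then rebuilds the route by splicing the maze's cells in at InsertIndex in place of RemoveCount original cells.
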(event EventBeginPlay)

(event Collision|EventActorBeginOverlap
  (params (OtherActor :type Actor%20Object%20Reference)))

(event EventTick
  (params (DeltaSeconds :type Float%20%28single-precision%29)))

(fn ConstructionScript)

(fn GetCellbyNumber
  (params (Number :type Integer))
  (return (Utilities|Array|Get(acopy) (Variables|Default|GetCells) Number)))

(fn GetNextCelltoMove
  (params (CellNumber :type Integer))
  (return (Math|Integer|%(Integer) CellNumber (Utilities|Array|Length (Variables|Default|GetCells)))))

(fn UpdateParkour
  (Default|DisplayMazePath (Variables|Default|GetMazePath))
  (bind _output_get (LocalVariables|SetNewSize (+ (- (Utilities|Array|Length (Variables|Default|GetCells)) (LocalVariables|GetRemoveCount)) (Utilities|Array|Length (Variables|/Game/Blueprints/Gameplay/BP_MazePath.BP_MazePath_C|GetListOfCells (Variables|Default|GetMazePath))))))
  (for _index (range 0 _output_get)
    (if (< _index (LocalVariables|GetInsertIndex))
      (Utilities|Array|SetArrayElem (LocalVariables|GetNewCells) _index (Utilities|Array|Get(acopy) (Variables|Default|GetCells) _index))
      (elif (< _index (+ (LocalVariables|GetInsertIndex) (Utilities|Array|Length (Variables|/Game/Blueprints/Gameplay/BP_MazePath.BP_MazePath_C|GetListOfCells (Variables|Default|GetMazePath)))))
        (Utilities|Array|SetArrayElem (LocalVariables|GetNewCells) _index (Utilities|Array|Get(acopy) (Variables|/Game/Blueprints/Gameplay/BP_MazePath.BP_MazePath_C|GetListOfCells (Variables|Default|GetMazePath)) (- _index (LocalVariables|GetInsertIndex))))
        (else
          (Utilities|Array|SetArrayElem (LocalVariables|GetNewCells) _index (Utilities|Array|Get(acopy) (Variables|Default|GetCells) (+ (- _index (Utilities|Array|Length (Variables|/Game/Blueprints/Gameplay/BP_MazePath.BP_MazePath_C|GetListOfCells (Variables|Default|GetMazePath)))) (LocalVariables|GetRemoveCount))))))))
  (Variables|Default|SetCells (LocalVariables|GetNewCells)))