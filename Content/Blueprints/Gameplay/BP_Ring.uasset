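; BP_Ring is a ring pickup that records on the game instance that the player has the ring.
; BeginPlay caches the BP_LoopGameInstance, and a Box overlap by BP_ThirdPersonCharacter sets its HasRing flag.
; The pickup then calls SetActive(false), which hides the Cube and disables Box and Cube collision instead of destroying the actor.
; SetActive(true) restores both, though nothing in this Blueprint calls it.
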(event OnComponentBeginOverlap(Box)
  (params (OverlappedComponent :type Primitive%20Component%20Object%20Reference) (OtherActor :type Actor%20Object%20Reference) (OtherComp :type Primitive%20Component%20Object%20Reference) (OtherBodyIndex :type Integer) (bFromSweep :type Boolean) (SweepResult :type Hit%20Result%20Structure%20%28by%20ref%29))
  (Utilities|Casting|CastToBP_ThirdPersonCharacter OtherActor)
  (Variables|/Game/Blueprints/Global/BP_LoopGameInstance.BP_LoopGameInstance_C|SetHasRing (Variables|Default|GetAs%20BP%20Loop%20Game%20Instance) true)
  (CallFunction|SetActive false))

(event EventBeginPlay
  (bind _asbp_loop_game_instance (Utilities|Casting|CastToBP_LoopGameInstance (Game|GetGameInstance)))
  (Variables|Default|SetAs%20BP%20Loop%20Game%20Instance _asbp_loop_game_instance))

(event Collision|EventActorBeginOverlap
  (params (OtherActor :type Actor%20Object%20Reference)))

(event EventTick
  (params (DeltaSeconds :type Float%20%28single-precision%29)))

(fn ConstructionScript)

(fn SetActive
  (params (Active :type Boolean))
  (if Active
    (Collision|SetCollisionEnabled (Variables|Default|GetBox) "QueryAndPhysics")
    (Collision|SetCollisionEnabled (Variables|Default|GetCube) "QueryAndPhysics")
    (Rendering|SetVisibility (Variables|Default|GetCube) true false)
    (else
      (Collision|SetCollisionEnabled (Variables|Default|GetBox) "NoCollision")
      (Collision|SetCollisionEnabled (Variables|Default|GetCube) "NoCollision")
      (Rendering|SetVisibility (Variables|Default|GetCube) false false))))