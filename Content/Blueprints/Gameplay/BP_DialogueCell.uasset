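; BP_DialogueCell is a dialogue actor that shows character lines on screen in place of the player HUD.
; Activate hands the game instance to BPCDialogueComponent, which supplies the current row, branched by quest state, to the pawn's dialogue widget.
; Update advances rows, rechecking quest state and calling EndDialogue when the dialogue is finished.
; Desactivate removes the dialogue widget and restores the HUD.
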(event EventBeginPlay
  (|CallParentFunction) ; This node is disabled and will not be called.\nDrag off pins to build functionality.
)

(event Collision|EventActorBeginOverlap
  (params (OtherActor :type Actor%20Object%20Reference))
  (|CallParentFunction OtherActor) ; This node is disabled and will not be called.\nDrag off pins to build functionality.
)

(event EventTick
  (params (DeltaSeconds :type Float%20%28single-precision%29))
  (|CallParentFunction DeltaSeconds) ; This node is disabled and will not be called.\nDrag off pins to build functionality.
)

(event EventActivate
  (params (Pawn :type BP%20Player%20Pawn%20Object%20Reference))
  (bind _wbp_dialogueref (Variables|/Game/Blueprints/Gameplay/BP_PlayerPawn.BP_PlayerPawn_C|GetWBP_DialogueRef Pawn))
  (Variables|/Game/Blueprints/Global/Components/BPC_DialogueComponent.BPC_DialogueComponent_C|SetGameInstanceRef (Variables|Default|GetBPC_DialogueComponent) (Variables|/Game/Blueprints/Gameplay/BP_PlayerPawn.BP_PlayerPawn_C|GetAs%20BP%20Loop%20Game%20Instance Pawn))
  (Widget|RemovefromParent (Variables|/Game/Blueprints/Gameplay/BP_PlayerPawn.BP_PlayerPawn_C|GetPlayerHUD Pawn))
  (Default|GetCurrentDialogueRow (Variables|Default|GetBPC_DialogueComponent))
  (bind _true (Default|CheckQuestState (Variables|Default|GetBPC_DialogueComponent)))
  (if _true
    (Default|ReadNextRowbyCondition (Variables|Default|GetBPC_DialogueComponent)))
  (bind _charactername (Default|GetCharacterfromCurrentRow (Variables|Default|GetBPC_DialogueComponent)))
  (bind _dialoguelong (Default|GetDialogueLongfromCurrentRow (Variables|Default|GetBPC_DialogueComponent)))
  (Default|UpdateDialogue _wbp_dialogueref _charactername _dialoguelong)
  (UserInterface|Viewport|AddtoPlayerScreen _wbp_dialogueref))

(event EventUpdate
  (params (Pawn :type BP%20Player%20Pawn%20Object%20Reference))
  (bind _wbp_dialogueref (Variables|/Game/Blueprints/Gameplay/BP_PlayerPawn.BP_PlayerPawn_C|GetWBP_DialogueRef Pawn))
  (bind _isfinished (Default|IsDialogueFinished (Variables|Default|GetBPC_DialogueComponent)))
  (if _isfinished
    (bind _true (Default|CheckQuestState (Variables|Default|GetBPC_DialogueComponent)))
    (if _true
      (Default|ReadNextRowbyCondition (Variables|Default|GetBPC_DialogueComponent))
      (else
        (Default|ReadNextRow (Variables|Default|GetBPC_DialogueComponent))))
    (bind _charactername (Default|GetCharacterfromCurrentRow (Variables|Default|GetBPC_DialogueComponent)))
    (bind _dialoguelong (Default|GetDialogueLongfromCurrentRow (Variables|Default|GetBPC_DialogueComponent)))
    (Default|UpdateDialogue _wbp_dialogueref _charactername _dialoguelong)
    (Default|EndDialogue _wbp_dialogueref)
    (else
      (Default|ReadNextRow (Variables|Default|GetBPC_DialogueComponent))
      (bind _charactername_2 (Default|GetCharacterfromCurrentRow (Variables|Default|GetBPC_DialogueComponent)))
      (bind _dialoguelong_2 (Default|GetDialogueLongfromCurrentRow (Variables|Default|GetBPC_DialogueComponent)))
      (Default|UpdateDialogue _wbp_dialogueref _charactername_2 _dialoguelong_2))))

(event EventDesactivate
  (params (Pawn :type BP%20Player%20Pawn%20Object%20Reference))
  (Widget|RemovefromParent (Variables|/Game/Blueprints/Gameplay/BP_PlayerPawn.BP_PlayerPawn_C|GetWBP_DialogueRef Pawn))
  (UserInterface|Viewport|AddtoPlayerScreen (Variables|/Game/Blueprints/Gameplay/BP_PlayerPawn.BP_PlayerPawn_C|GetPlayerHUD Pawn)))

(fn ConstructionScript
  (|CallParentFunction))