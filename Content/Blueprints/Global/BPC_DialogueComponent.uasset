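; BPC_DialogueComponent is a component that steps through a linear dialogue stored in a data table.
; It looks up rows by number converted to a row name, caches the current row, and exposes its long text and character.
; Each row's NextRow index drives advancing, and a negative value marks the dialogue as finished.
; Resetting sets the row number back to zero without reloading the cached row.
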(fn GetCurrentDialogueRow
  (bind _returnvalue (Utilities|GetDataTableRow (Variables|Default|GetDialogueDataTable) (Utilities|String|StringToName (Utilities|String|ToString(Integer) (Variables|Default|GetCurrentRowNumber))))
    (:then
      (bind _output_get (Variables|Default|SetCurrentDialogueRow _returnvalue))
      (return _output_get))))

(fn GetDialogueLongfromCurrentRow
  (return (.DialogueLong (Utilities|Struct|BreakST_DialogueRowDatas (Variables|Default|GetCurrentDialogueRow)))))

(fn GetCharacterfromCurrentRow
  (return (.Character (Utilities|Struct|BreakST_DialogueRowDatas (Variables|Default|GetCurrentDialogueRow)))))

(fn IsDialogueFinished
  (return (< (.NextRow (Utilities|Struct|BreakST_DialogueRowDatas (Variables|Default|GetCurrentDialogueRow))) 0)))

(fn ReadNextRow
  (Variables|Default|SetCurrentRowNumber (.NextRow (Utilities|Struct|BreakST_DialogueRowDatas (Variables|Default|GetCurrentDialogueRow))))
  (CallFunction|GetCurrentDialogueRow))

(fn ResetDialogueData
  (Variables|Default|SetCurrentRowNumber 0))