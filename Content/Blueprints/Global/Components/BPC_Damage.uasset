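; BPC_Damage is an actor component that handles health and attacks in fights between the player and monsters.
; DealDamage hits another damage component with Attack, then starts a one-second cooldown timed on Tick.
; TakeDamage lowers Health and, for the player, copies it to PlayerHealth in the loop game instance.
; At zero health, Death calls the player's or monster's Death, then tells FightingCell the fight is over.
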(event EventBeginPlay)

(event EventTick
  (params (DeltaSeconds :type Float%20%28single-precision%29))
  (if (Variables|Default|GetAttackCooldown)
    (Variables|Default|SetTimer (+ (Variables|Default|GetTimer) DeltaSeconds)))
  (if (>= (Variables|Default|GetTimer) 1.0)
    (Variables|Default|SetTimer 0.0)
    (Variables|Default|SetAttackCooldown false)))

(fn DealDamage
  (params (BPC_Damage :type BPC%20Damage%20Object%20Reference))
  (if (not (Variables|Default|GetAttackCooldown))
    (Variables|Default|SetAttackCooldown true)
    (CallFunction|TakeDamage BPC_Damage (Variables|Default|GetAttack))))

(fn TakeDamage
  (params (Amount :type Float%20%28double-precision%29))
  (bind _playerref (Variables|Default|GetPlayerRef))
  (bind _output_get (Variables|Default|SetHealth (- (Variables|Default|GetHealth) Amount)))
  (Utilities|IsValid _playerref
    (:Is%20Valid
      (Variables|/Game/Blueprints/Global/BP_LoopGameInstance.BP_LoopGameInstance_C|SetPlayerHealth (Variables|/Game/Blueprints/Gameplay/BP_PlayerPawn.BP_PlayerPawn_C|GetAs%20BP%20Loop%20Game%20Instance _playerref) (Variables|Default|GetHealth)))
    (:Is%20Not%20Valid
      _))
  (if (<= _output_get 0.0)
    (CallFunction|Death)))

(fn Death
  (Utilities|IsValid (Variables|Default|GetPlayerRef)
    (:Is%20Valid
      (Default|Death (Variables|Default|GetPlayerRef)))
    (:Is%20Not%20Valid
      (Utilities|IsValid (Variables|Default|GetMonsterRef)
        (:Is%20Valid
          (Default|Death (Variables|Default|GetMonsterRef))))))
  (Default|FightOver (Variables|Default|GetFightingCell)))