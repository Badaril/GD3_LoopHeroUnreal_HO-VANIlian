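; Game mode Blueprint that provides load and save functions for the "LoopSave" slot.
; BeginPlay caches a reference to BP_LoopGameInstance, but calls neither function.
; LoadGame stores the existing BP_SaveGame, or calls SaveGame when none exists.
; SaveGame always creates a fresh save object, copies its game data into the game instance rather than the reverse, then writes it to the slot.
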(event EventBeginPlay
  (bind _asbp_loop_game_instance (Utilities|Casting|CastToBP_LoopGameInstance (Game|GetGameInstance)))
  (Variables|Default|SetAs%20BP%20Loop%20Game%20Instance _asbp_loop_game_instance))

(event EventTick
  (params (DeltaSeconds :type Float%20%28single-precision%29)))

(fn ConstructionScript)

(fn LoadGame
  (bind _returnvalue (SaveGame|DoesSaveGameExist "LoopSave"))
  (if _returnvalue
    (bind _returnvalue_2 (SaveGame|LoadGamefromSlot "LoopSave"))
    (bind _asbp_save_game (Utilities|Casting|CastToBP_SaveGame _returnvalue_2))
    (Variables|Default|SetBP_SaveGame _asbp_save_game)
    (else
      (CallFunction|SaveGame))))

(fn SaveGame
  (bind _returnvalue (SaveGame|CreateSaveGameObject "/Game/Blueprints/Global/BP_SaveGame.BP_SaveGame_C"))
  (bind _output_get (Variables|Default|SetBP_SaveGame _returnvalue))
  (Variables|/Game/Blueprints/Global/BP_LoopGameInstance.BP_LoopGameInstance_C|SetST_GameDatas (Variables|Default|GetAs%20BP%20Loop%20Game%20Instance) (Variables|/Game/Blueprints/Global/BP_SaveGame.BP_SaveGame_C|GetST_GameDatas _output_get))
  (SaveGame|SaveGametoSlot _output_get "LoopSave"))